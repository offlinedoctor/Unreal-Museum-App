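; BP_PlayerPawn is the player pawn that lets the user click exhibit pieces to view their details.
; BeginPlay enables the mouse cursor and creates a collapsed Umg_ExhibitDetails widget.
; A left click traces under the cursor: a BP_ExhibitPiece hit shows the widget with its name and description and passes its Actorname to CamObjectRef.SetAllHidden.
; Any other click collapses the widget.
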(event `self.ReceiveBeginPlay`
  (bind _returnvalue (`GameplayStatics.GetPlayerController` 0))
  (set `PlayerController.bShowMouseCursor` true _returnvalue)
  (set `PlayerController.bEnableMouseOverEvents` true _returnvalue)
  (bind _returnvalue_2 (`|CreateWidget` "/Game/Blueprints/UMG/umg_ExhibitDetails.umg_ExhibitDetails_C"))
  (bind _output_get (set `self.NewVar_0` _returnvalue_2))
  (`UserWidget.AddToViewport` _output_get 0)
  (`Widget.SetVisibility` (`self.NewVar_0`) "Collapsed"))

(event `Key|LeftMouseButton`
  (params (Key :type "Key Structure"))
  (bind _newvar_0 (`self.NewVar_0`))
  (bind (_bblockinghit _binitialoverlap _time _distance _location _impactpoint _normal _impactnormal _physmat _hitactor) (`GameplayStatics.BreakHitResult` (`PlayerController.GetHitResultUnderCursorByChannel` (`GameplayStatics.GetPlayerController` 0) "TraceTypeQuery1" true)))
  (:`Pressed`
    (if (`KismetMathLibrary.ClassIsChildOf` (`GameplayStatics.GetObjectClass` _hitactor) "/Game/Blueprints/ExhibitItems/BP_ExhibitPiece.BP_ExhibitPiece_C")
      (`Widget.SetVisibility` (`self.NewVar_0`) "Visible")
      (bind _asbp_exhibit_piece (cast `/Game/Blueprints/ExhibitItems/BP_ExhibitPiece` _hitactor))
      (`TextBlock.SetText` (`/Game/Blueprints/UMG/umg_ExhibitDetails.artName` _newvar_0) (`KismetTextLibrary.Conv_StringToText` (`/Game/Blueprints/ExhibitItems/BP_ExhibitPiece.name` _asbp_exhibit_piece)))
      (`TextBlock.SetText` (`/Game/Blueprints/UMG/umg_ExhibitDetails.artDesc` _newvar_0) (`KismetTextLibrary.Conv_StringToText` (`/Game/Blueprints/ExhibitItems/BP_ExhibitPiece.description` _asbp_exhibit_piece)))
      (`/Game/Blueprints/ObjectRotating/CamActor.SetAllHidden` (`self.camObjectRef`) (`/Game/Blueprints/ExhibitItems/BP_ExhibitPiece.actorname` _asbp_exhibit_piece))
      (else
        (`Widget.SetVisibility` (`self.NewVar_0`) "Collapsed")))))

(fn `UserConstructionScript`)