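; CamActor is a preview actor that shows one of four spinning display models to a SceneCaptureComponent2D.
; The construction script restricts the capture to this actor alone, isolating the models from the rest of the level.
; Tick adds a fixed local rotation to StaticMesh, VastLand, Chess and Scene2 each frame, without delta-time scaling.
; SetAllHidden takes a name string, shows the matching model and hides the other three.
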(event `self.ReceiveTick`
  (params (DeltaSeconds :type "Float (single-precision)"))
  (`SceneComponent.K2_AddLocalRotation` (`self.StaticMesh`) (struct :`Yaw` 0.5) false false)
  (`SceneComponent.K2_AddLocalRotation` (`self.vastLand`) (struct :`Yaw` 0.5) false false)
  (`SceneComponent.K2_AddLocalRotation` (`self.chess`) (struct :`Yaw` 0.5) false false)
  (`SceneComponent.K2_AddLocalRotation` (`self.Scene2`) (struct :`Yaw` 0.5) false false))

(event `SetAllHidden`
  (params (string :type String))
  (switch `string` string
    (:`vastland`
      (`SceneComponent.SetVisibility` (`self.vastLand`) true false)
      (`SceneComponent.SetVisibility` (`self.chess`) false false)
      (`SceneComponent.SetVisibility` (`self.dragonStatue`) false false)
      (`SceneComponent.SetVisibility` (`self.StaticMesh`) false false))
    (:`chess`
      (`SceneComponent.SetVisibility` (`self.chess`) true false)
      (`SceneComponent.SetVisibility` (`self.vastLand`) false false)
      (`SceneComponent.SetVisibility` (`self.dragonStatue`) false false)
      (`SceneComponent.SetVisibility` (`self.StaticMesh`) false false))
    (:`dragonstatue`
      (`SceneComponent.SetVisibility` (`self.dragonStatue`) true false)
      (`SceneComponent.SetVisibility` (`self.vastLand`) false false)
      (`SceneComponent.SetVisibility` (`self.chess`) false false)
      (`SceneComponent.SetVisibility` (`self.StaticMesh`) false false))
    (:`monkeycrown`
      (`SceneComponent.SetVisibility` (`self.StaticMesh`) true false)
      (`SceneComponent.SetVisibility` (`self.vastLand`) false false)
      (`SceneComponent.SetVisibility` (`self.chess`) false false)
      (`SceneComponent.SetVisibility` (`self.dragonStatue`) false false))))

(fn `UserConstructionScript`
  (set `SceneCaptureComponent.ShowOnlyActors` (`|MakeArray` self :!type "Actor Object Reference") (`self.SceneCaptureComponent2D`)))